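; BP_Skill_FireStorm is an area-of-effect skill actor in the skill system, built on a parent skill class's StartCast and Cast events.
; StartCast only forwards the target location and object to the parent.
; Cast calls the parent, moves a component (apparently the particle) to the target location as a relative location over a short fixed time, prints a debug message and destroys the actor.
; The file shows no damage or area logic.
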(event EventBeginPlay
  (|CallParentFunction) ; This node is disabled and will not be called.\nDrag off pins to build functionality.
)

(event Collision|EventActorBeginOverlap
  (params (OtherActor :type Actor%20Object%20Reference))
  (|CallParentFunction OtherActor) ; This node is disabled and will not be called.\nDrag off pins to build functionality.
)

(event EventTick
  (params (DeltaSeconds :type Float%20%28single-precision%29))
  (|CallParentFunction DeltaSeconds) ; This node is disabled and will not be called.\nDrag off pins to build functionality.
)

(event EventStartCast
  (params (TargetLocation :type Vector :default "0, 0, 0") (TargetObject :type BP%20Target%20Object%20Reference))
  (|CallParentFunction TargetLocation TargetObject))

(event EventCast
  (|CallParentFunction)
  (Components|MoveComponentTo 0 (stale EventStartCast TargetLocation) "0, 0, 0" false false 2.0 false)
  (Development|PrintString "Particle Moved")
  (Actor|DestroyActor))

(fn ConstructionScript
  (|CallParentFunction))