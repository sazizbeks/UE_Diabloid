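; Actor component, going by its name, that tracks a character's experience, level and skill points for the skill system.
; Setup on BeginPlay loads the level's DT_Experience row, keyed by level number, falling back to the first level.
; AddExp walks rows until experience fits, clamps at MaxLevel and awards a point per level gained through AddSkillPoints, which fires an event.
; IncreaseLevel jumps levels directly, granting points without that event; an older AddExp version remains unconnected.
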(event EventBeginPlay
  (CallFunction|Setup))

(fn AddExp
  (params (ExpToAdd :type Integer))
  (if (and (> ExpToAdd 0) (!= (.level (Variables|Default|GetLevelInfo)) (Variables|Default|GetMaxLevel)))
    (bind _output_get (Variables|Default|SetActualExperience (+ (Variables|Default|GetActualExperience) ExpToAdd)))
    (LocalVariables|SetActualLevel (.level (Variables|Default|GetLevelInfo))) ; Needed to futher calculation
    (if (>= _output_get (.maxexp (Variables|Default|GetLevelInfo)))
      (while (and (Math|Boolean|NORBoolean (Math|Integer|InRange(Integer) (Variables|Default|GetActualExperience) (.minexp (Variables|Default|GetLevelInfo)) (.maxexp (Variables|Default|GetLevelInfo)) true false) (LocalVariables|GetExpIsAboveMaxLevel)) (< (.level (Variables|Default|GetLevelInfo)) (Variables|Default|GetMaxLevel)))
        (bind _returnvalue (Utilities|GetDataTableRow "/Game/SkillSystem/DataTables/DT_Experience.DT_Experience" (Utilities|String|StringToName (Utilities|String|ToString(Integer) (+ (.level (Variables|Default|GetLevelInfo)) 1))))
          (:then
            (Variables|Default|SetLevelInfo _returnvalue))
          (:RowNotFound
            (LocalVariables|SetExpIsAboveMaxLevel true))))
      (bind _output_get_2 (LocalVariables|SetExpIsAboveMaxLevel (Math|Boolean|ORBoolean (LocalVariables|GetExpIsAboveMaxLevel) (>= (Variables|Default|GetActualExperience) (.maxexp (Variables|Default|GetLevelInfo))) (== (.level (Variables|Default|GetLevelInfo)) (Variables|Default|GetMaxLevel)))))
      (if _output_get_2
        (bind _returnvalue_2 (Utilities|GetDataTableRow "/Game/SkillSystem/DataTables/DT_Experience.DT_Experience" (Utilities|String|StringToName (Utilities|String|ToString(Integer) (Variables|Default|GetMaxLevel))))
          (:then
            (Variables|Default|SetLevelInfo _returnvalue_2)
            (Variables|Default|SetActualExperience (.maxexp (Variables|Default|GetLevelInfo))))
          (:RowNotFound
            _)))
      (CallFunction|AddSkillPoints (- (.level (Variables|Default|GetLevelInfo)) (LocalVariables|GetActualLevel))))))

(fn IncreaseLevel
  (params (LevelsToAdd :type Integer))
  (if (> LevelsToAdd 0)
    (bind _output_get (LocalVariables|SetFinalLevel (+ (.Level (Utilities|Struct|BreakBPS_PlayerExperience (Variables|Default|GetLevelInfo))) LevelsToAdd)))
    (bind _returnvalue (Utilities|GetDataTableRow "/Game/SkillSystem/DataTables/DT_Experience.DT_Experience" (Utilities|String|StringToName (Utilities|String|ToString(Integer) _output_get)))
      (:then
        (Variables|Default|SetSkillPoints (+ (- (.Level (Utilities|Struct|BreakBPS_PlayerExperience _returnvalue)) (.level (Variables|Default|GetLevelInfo))) (Variables|Default|GetSkillPoints)))
        (bind _output_get_2 (Variables|Default|SetLevelInfo _returnvalue))
        (Variables|Default|SetActualExperience (.MinExp (Utilities|Struct|BreakBPS_PlayerExperience _output_get_2))))
      (:RowNotFound
        (bind _lastlevel (CallFunction|GetLastLevel))
        (if (not (== (.Level (Utilities|Struct|BreakBPS_PlayerExperience _lastlevel)) (.Level (Utilities|Struct|BreakBPS_PlayerExperience (Variables|Default|GetLevelInfo)))))
          (bind _output_get_3 (Variables|Default|SetLevelInfo _lastlevel))
          (bind _output_get_4 (LocalVariables|SetLastLevel _output_get_3))
          (Variables|Default|SetActualExperience (.maxexp _output_get_4)))))))

(fn Setup
  (if (not (Variables|Default|GetIsSetUp))
    (bind _returnvalue (Utilities|GetDataTableRow "/Game/SkillSystem/DataTables/DT_Experience.DT_Experience" (Utilities|String|StringToName (Utilities|String|ToString(Integer) (.level (Variables|Default|GetLevelInfo)))))
      (:then
        (bind _output_get (Variables|Default|SetLevelInfo _returnvalue))
        (Variables|Default|SetActualExperience (.minexp _output_get)))
      (:RowNotFound
        (bind _firstlevel (CallFunction|GetFirstLevel))
        (bind _output_get_2 (Variables|Default|SetLevelInfo _firstlevel))
        (Variables|Default|SetActualExperience (.minexp _output_get_2))))
    (Variables|Default|SetIsSetUp true)))

(fn AddSkillPoints
  (params (SkillPointsToAdd :type Integer))
  (Variables|Default|SetSkillPoints (+ SkillPointsToAdd (Variables|Default|GetSkillPoints)))
  (Default|CallAddSkillPointsEvent))

(fn DecreaseSkillPoints
  (params (SkillPoints :type Integer))
  (if (<= SkillPoints (Variables|Default|GetSkillPoints))
    (bind _result (Utilities|NegateInt SkillPoints)
      (:%20%20
        (CallFunction|AddSkillPoints _result)))))