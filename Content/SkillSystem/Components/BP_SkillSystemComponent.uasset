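; Skill system component that tracks a character's unlocked skills and their tiers, and casts them.
; AddSkill checks the skill's DT_Skill row, unlocks it at tier 1 or raises it up to MaxTier in the SkillUnlocks map, then fires the AddSkill event.
; CastSkill confirms the unlock through QuerySkill, spawns the skill's specific Blueprint actor at the owner's transform and calls StartCast with the target.
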(event EventBeginPlay)

(event EventTick
  (params (DeltaSeconds :type Float%20%28single-precision%29)))

(fn AddSkill
  (params (RowName :type Name))
  (bind _skillunlocks (Variables|Default|GetSkillUnlocks))
  (bind (_value _returnvalue) (Utilities|Map|Find _skillunlocks RowName))
  (bind _returnvalue_2 (Utilities|GetDataTableRow "/Game/SkillSystem/DataTables/DT_Skill.DT_Skill" RowName)
    (:then
      (LocalVariables|SetSkillInfo _returnvalue_2)
      (if _returnvalue
        (LocalVariables|SetFoundSkillTier _value)
        (if (< (LocalVariables|GetFoundSkillTier) (.MaxTier (Utilities|Struct|BreakBPS_Skill (LocalVariables|GetSkillInfo))))
          (bind _result (Math|Integer|IncrementInt (LocalVariables|GetFoundSkillTier))
            (:%20%20
              (Utilities|Map|Add (Variables|Default|GetSkillUnlocks) RowName _result)
              (Default|CallAddSkillEvent (LocalVariables|GetSkillInfo))
              (return true)))
          (else
            (return false)))
        (else
          (Utilities|Map|Add (Variables|Default|GetSkillUnlocks) RowName 1)
          (Default|CallAddSkillEvent (LocalVariables|GetSkillInfo))
          (return true))))))

(fn QuerySkill
  (params (RowName :type Name))
  (bind _skillunlocks (Variables|Default|GetSkillUnlocks))
  (bind (_value _returnvalue) (Utilities|Map|Find _skillunlocks RowName))
  (return _returnvalue (Math|Integer|SelectInt _value 0 _returnvalue)))

(fn CastSkill
  (params (SkillInfo :type BPS%20Skill%20Structure) (TargetLocation :type Vector) (TargetObject :type BP%20Target%20Object%20Reference) (Owner :type BP%20Base%20Character%20Object%20Reference))
  (bind (_skillrowname _name _description _needtarget _needlocation _cooldown _manacost _maxtier _casttime _requiredskillpoints _specificblueprint) (Utilities|Struct|BreakBPS_Skill SkillInfo))
  (bind _found (CallFunction|QuerySkill _skillrowname))
  (if _found
    (bind _returnvalue (Game|SpawnActorfromClass _specificblueprint (Transformation|GetActorTransform Owner) "Undefined" Owner _skillrowname 0))
    (Default|StartCast _returnvalue TargetLocation TargetObject)))